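; BP_FlashStaticMesh is an actor that shows a given static mesh with a looping flash effect.
; Its SetStaticMesh event assigns the mesh and replaces every material slot with a dynamic instance of Mat_Flash, stored in an array.
; A looping timeline then writes the Color variable, with the timeline's alpha as the A channel, into each instance's Color parameter on every update.
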(event `SetStaticMesh`
  (params (StaticMesh :type "StaticMesh Object Reference"))
  (bind _matinstance (`self.MatInstance`))
  (bind _staticmeshcomponent (`self.StaticMeshComponent`))
  (bind (_color_x _color_y _color_z) (`KismetMathLibrary.BreakVector` (`self.Color`)))
  (`StaticMeshComponent.SetStaticMesh` _staticmeshcomponent StaticMesh)
  (for _index (range (+ (`PrimitiveComponent.GetNumMaterials` _staticmeshcomponent) 1))
    (bind _returnvalue (`PrimitiveComponent.CreateDynamicMaterialInstance` _staticmeshcomponent _index "/Game/Main/Materials/Mat_Flash.Mat_Flash" "None"))
    (`KismetArrayLibrary.Array_Add` _matinstance _returnvalue))
  (`TimelineComponent.SetLooping` (`self.FlashTimeline`) true)
  (bind (_direction _alpha) (`Timeline|FlashTimeline`)
    (:`Update`
      (for _array_element _matinstance
        (`MaterialInstanceDynamic.SetVectorParameterValue` _array_element "Color" (make `LinearColor` _color_x _color_y _color_z _alpha))))))

(fn `UserConstructionScript`)