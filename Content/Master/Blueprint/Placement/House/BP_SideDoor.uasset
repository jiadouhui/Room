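; A side door Blueprint for house placement that slides open when something overlaps its trigger.
; A timeline lerps the door's relative X location despite angle-named variables, and reverses when the overlap ends.
; A gate blocks opening between StartMove and StopMove, which extend the parent's move handling, while closing stays ungated.
; On BeginPlay it also casts FlashDoor to FlashMaterials.
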(event `self.ReceiveBeginPlay`
  (`parent.ReceiveBeginPlay`)
  (`self.CastToFlashMaterials` (`self.FlashDoor`)))

(event `self.Trigger.OnComponentBeginOverlap`
  (params (OverlappedComponent :type "PrimitiveComponent Object Reference") (OtherActor :type "Actor Object Reference") (OtherComp :type "PrimitiveComponent Object Reference") (OtherBodyIndex :type Integer) (bFromSweep :type Boolean) (SweepResult :type "HitResult Structure (by ref)"))
  (`/Engine/EditorBlueprintResources/StandardMacros.Gate` false :!label _label
    (:`Exit`
      (bind (_direction _program) (`Timeline|RotateTime` :!label _label_2)
        (:`Update`
          (`SceneComponent.K2_SetRelativeLocation` (`self.Door`) (`KismetMathLibrary.MakeVector` (`KismetMathLibrary.Lerp` (`self.StartAngle`) (`self.TargetAngle`) _program)) false false))))))

(event `self.StopMove`
  (`parent.StopMove`)
  (goto _label :!via `Open`))

(event `self.StartMove`
  (`parent.StartMove`)
  (goto _label :!via `Close`))

(event `self.Trigger.OnComponentEndOverlap`
  (params (OverlappedComponent :type "PrimitiveComponent Object Reference") (OtherActor :type "Actor Object Reference") (OtherComp :type "PrimitiveComponent Object Reference") (OtherBodyIndex :type Integer))
  (goto _label_2 :!via `Reverse`))

(fn `UserConstructionScript`
  (`parent.UserConstructionScript`))