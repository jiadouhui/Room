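; BP_Interactivable is an interactable actor that can flash as a highlight and render its mesh for UI display.
; FlashMesh copies StaticMesh with dynamic flash materials, and SetFlashEnable toggles its visibility and a looping timeline that animates their color alpha.
; RenderCamera captures only this actor's mesh, and GetRenderUIMaterial points it at a new render target, returning a dynamic UI material that shows the result.
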(event `self.ReceiveBeginPlay`
  (bind _flashmesh (`self.FlashMesh`))
  (`StaticMeshComponent.SetStaticMesh` _flashmesh (`StaticMeshComponent.StaticMesh` (`self.StaticMesh`)))
  (for _index (range (+ (`PrimitiveComponent.GetNumMaterials` _flashmesh) 1))
    (bind _returnvalue (`PrimitiveComponent.CreateDynamicMaterialInstance` _flashmesh _index "/Game/Master/Materials/Mat_Flash.Mat_Flash" "None"))
    (`KismetArrayLibrary.Array_Add` (`self.Materials`) _returnvalue)
    (`TimelineComponent.SetLooping` (`self.FlashTime`) true)))

(event `SetFlashEnable`
  (params (Enable :type Boolean))
  (bind (_flashcolor_r _flashcolor_g _flashcolor_b) (break `LinearColor` (`self.FlashColor`)))
  (`SceneComponent.SetHiddenInGame` (`self.FlashMesh`) (not Enable) false)
  (if Enable
    (bind (_direction _alpha) (`Timeline|FlashTime` :!label _label)
      (:`Update`
        (for _array_element (`self.Materials`)
          (`MaterialInstanceDynamic.SetVectorParameterValue` _array_element "Color" (make `LinearColor` _flashcolor_r _flashcolor_g _flashcolor_b _alpha)))))
    (else
      (goto _label :!via `Stop`))))

(fn `GetRenderUIMaterial`
  (returns (Value :type "MaterialInterface Object Reference"))
  (bind _returnvalue (`KismetRenderingLibrary.CreateRenderTarget2D` 1080 1080 "RTF_RGBA32f"))
  (bind _output_get (set `SceneCaptureComponent2D.TextureTarget` _returnvalue (`self.RenderCamera`)))
  (bind _returnvalue_2 (`KismetMaterialLibrary.CreateDynamicMaterialInstance` "/Game/Master/Materials/Mat_UI.Mat_UI"))
  (`MaterialInstanceDynamic.SetTextureParameterValue` _returnvalue_2 "RenderTarget" _output_get)
  (return _returnvalue_2))

(fn `UserConstructionScript`
  (bind _rendercamera (`self.RenderCamera`))
  (set `SceneCaptureComponent.ShowOnlyActors` (`|MakeArray` self :!type "Actor Object Reference") _rendercamera)
  (`SceneCaptureComponent.ShowOnlyComponent` _rendercamera (`self.StaticMesh`)))