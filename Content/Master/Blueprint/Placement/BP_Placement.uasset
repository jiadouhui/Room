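; BP_Placement is a placeable object that can be moved and shows whether its current spot is valid.
; StartMove and StopMove toggle the moving state, flashing and static mesh collision.
; Each Tick, IsOverlapTarget compares the Occupied box's count of overlapping BP_Placement actors to an expected value, setting validity and a green or red flash color.
; BeginPlay slightly shrinks that box horizontally.
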(event `self.ReceiveBeginPlay`
  (bind _occupied (`self.Occupied`))
  (`parent.ReceiveBeginPlay`)
  (`BoxComponent.SetBoxExtent` _occupied (- (`BoxComponent.BoxExtent` _occupied) (1.0 1.0 0.0)) true))

(event `self.ReceiveTick`
  (params (DeltaSeconds :type "Float (single-precision)"))
  (bind _output_get (set `self.IsVaildPlace` (`self.IsOverlapTarget` (`self.Occupied`) "BP_Placement_C")))
  (set `self.FlashColor` (`KismetMathLibrary.SelectColor` (struct :`R` 0.188 :`G` 0.516 :`A` 1.0) (struct :`R` 0.995 :`A` 1.0) _output_get)))

(event `StartMove`
  (`self.SetFlashEnable` true)
  (`PrimitiveComponent.SetCollisionEnabled` (`self.StaticMesh`) "NoCollision")
  (set `self.IsMoving` true))

(event `StopMove`
  (`self.SetFlashEnable` false)
  (`PrimitiveComponent.SetCollisionEnabled` (`self.StaticMesh`) "QueryAndPhysics")
  (set `self.IsMoving` false))

(fn `IsOverlapTarget`
  (params (Target :type "PrimitiveComponent Object Reference") (ClassFilter :type "Actor Class Reference") (IgironSelf :type Boolean :default true))
  (returns (ReturnValue :type Boolean) (OverlappingActors :type "Array of Actor Object Reference"))
  (bind _overlappingactors (`PrimitiveComponent.GetOverlappingActors` Target ClassFilter))
  (return (== (`KismetArrayLibrary.Array_Length` _overlappingactors) (`KismetMathLibrary.SelectInt` 1 0 (`KismetMathLibrary.BooleanNAND` (`KismetArrayLibrary.Array_Contains` _overlappingactors (`self.GetOwner`)) IgironSelf))) _overlappingactors))

(fn `UserConstructionScript`)