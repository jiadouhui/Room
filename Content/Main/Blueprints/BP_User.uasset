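; Player pawn for grid-based object placement, with right-drag yaw and mouse-wheel spring-arm zoom.
; UserUI spawns placeables that follow a mouse-ray trace while BP_Floor grids show; left click places them, or destroys them if placement is invalid, and middle click rotates them 90°.
; Clicking a BP_Placeable0 shows its buttons, whose ControlMove event picks it up again and warps the cursor onto it.
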(event `self.ReceiveBeginPlay`
  ;[1 1 1] 生成UI
  (bind _returnvalue (`|CreateWidget` "/Game/Main/Blueprints/UI/BP_UserUI.BP_UserUI_C"))
  (bind _output_get (set `self.UserUI` _returnvalue))
  ;[1 1 1] 点击生成物品
  (add `/Game/Main/Blueprints/UI/BP_UserUI.OnSpawnPlaceable` _output_get (delegate `SpawnPlaceable`))
  (`EnhancedInputSubsystemInterface.AddMappingContext` (pcsubsystem `EnhancedInputLocalPlayerSubsystem` (`GameplayStatics.GetPlayerController` 0)) "/Game/Main/Input/IMC_Context.IMC_Context" 0 (struct)))

(event `SpawnPlaceable`
  (params (Target :type "/Game/Main/Blueprints/BP_Placeable0 Class Reference"))
  (bind _returnvalue_location (`KismetMathLibrary.BreakTransform` (`self.GetTransform`)))
  (bind (_returnvalue_x _returnvalue_y) (`KismetMathLibrary.BreakVector2D` (`WidgetLayoutLibrary.GetViewportSize`)))
  ;[1 1 1] 点击生成物品
  (`KismetSystemLibrary.Delay` 0.0)
  (bind _returnvalue (`|SpawnActorFromClass` Target (`KismetMathLibrary.MakeTransform` _returnvalue_location) "AlwaysSpawn" "SelectDefaultAtRuntime" null null))
  (`self.Control Target Move` _returnvalue)
  (`PlayerController.SetMouseLocation` (`GameplayStatics.GetPlayerController` 0) (`KismetMathLibrary.FTrunc` (* _returnvalue_x 0.5)) (`KismetMathLibrary.FTrunc` (* _returnvalue_y 0.7))))

(event `EnhancedInput|/Game/Main/Input/IA_Move`
  (params (ActionValue :type "Vector2D Structure") (ElapsedSeconds :type "Float (double-precision)") (TriggeredSeconds :type "Float (double-precision)") (InputAction :type "InputAction Object Reference" :default "/Game/Main/Input/IA_Move.IA_Move"))
  (:`Triggered`
    (`KismetSystemLibrary.PrintString` (`KismetStringLibrary.Conv_Vector2dToString` ActionValue))))

(event `EnhancedInput|/Game/Main/Input/IA_Fire`
  (params (ActionValue :type Boolean) (ElapsedSeconds :type "Float (double-precision)") (TriggeredSeconds :type "Float (double-precision)") (InputAction :type "InputAction Object Reference" :default "/Game/Main/Input/IA_Fire.IA_Fire"))
  (:`Triggered`
    (`KismetSystemLibrary.PrintString` "Hello")))

(event `Key|LeftMouseButton`
  (params (Key :type "Key Structure"))
  (bind (_originposition _endposition) (`self.GetMouseRay`))
  (bind _putactor (`self.PutActor`))
  (bind _seletactor (`self.SeletActor`))
  ;[1 1 1] 鼠标点击分支
  (:`Pressed`
    (`/Engine/EditorBlueprintResources/StandardMacros.IsValid` (`self.PutActor`)
      (:`Is Valid`
        ;;[1 1 1] 放置物品
        (`|ExecutionSequence`
          (:`then_0`
            (if (`/Game/Main/Blueprints/BP_Placeable0.GetCanPlace` _putactor)
              (`/Game/Main/Blueprints/BP_Placeable0.SetPlaced` _putactor true)
              (set `self.PutActor` null)
              (else
                (`self.K2_DestroyActor` _putactor))))
          (:`then_1`
            (`self.SetGripsVisiblity` false)
            (`Widget.SetVisibility` (`self.UserUI`) "Visible"))))
      (:`Is Not Valid`
        ;;[1 1 1] 按下放置的物品弹出按钮
        ;;;[1 1 1] 检测鼠标是否指向对象
        (bind _outhit (`KismetSystemLibrary.LineTraceSingle` _originposition _endposition "TraceTypeQuery3"))
        (bind _asbp_placeable (cast `/Game/Main/Blueprints/BP_Placeable0` (`.HitActor` (`GameplayStatics.BreakHitResult` _outhit)))
          (:`then`
            ;;;[1 1 1] 切换按钮的显示
            (`|ExecutionSequence`
              (:`then_0`
                (`/Engine/EditorBlueprintResources/StandardMacros.IsValid` _seletactor :!label _label
                  (:`Is Valid`
                    (`/Game/Main/Blueprints/BP_Placeable0.Set SelectBtnsIVisiblity ` _seletactor false (delegate `ControlMove`)) ; 关闭当前的按钮UI
                  )))
              (:`then_1`
                (bind _output_get (set `self.SeletActor` _asbp_placeable))
                (`/Game/Main/Blueprints/BP_Placeable0.Set SelectBtnsIVisiblity ` _output_get true (delegate `ControlMove`)) ; 开启当前的按钮UI
                (`Widget.SetVisibility` (`self.UserUI`) "Hidden"))))
          (:`CastFailed`
            (`Widget.SetVisibility` (`self.UserUI`) "Visible")
            (goto _label)))))))

(event `self.ReceiveTick`
  (params (DeltaSeconds :type "Float (single-precision)"))
  (bind (_originposition _endposition) (`self.GetMouseRay`))
  (bind _putactor (`self.PutActor`))
  ;[1 1 1] 控制移动对象
  ;;[1 1 1] 显示在格子上
  (`/Engine/EditorBlueprintResources/StandardMacros.IsValid` (`self.PutActor`)
    (:`Is Valid`
      (bind (_outhit _returnvalue) (`KismetSystemLibrary.LineTraceSingle` _originposition _endposition "TraceTypeQuery2"))
      (`/Game/Main/Blueprints/Placeables/BP_Floor.SetVisiblity` _putactor _returnvalue)
      (if _returnvalue
        (`self.K2_SetActorLocation` _putactor (- (`SceneComponent.K2_GetComponentLocation` (`.HitComponent` (`GameplayStatics.BreakHitResult` _outhit))) (0.0 0.0 10.0)) true true)))))

(event `ControlMove`
  (bind _seletactor (`self.SeletActor`))
  ;[1 1 1] 鼠标点击分支
  ;;[1 1 1] 按下放置的物品弹出按钮
  ;;;[1 1 1] 切换按钮的显示
  (`self.Control Target Move` _seletactor)
  (`self.Set Mouse To Actor` _seletactor))

(event `Key|MiddleMouseButton`
  (params (Key :type "Key Structure"))
  (bind _putactor (`self.PutActor`))
  ;[1 1 1] 控制移动对象
  ;;[1 1 1] 旋转对象
  (:`Pressed`
    (`/Engine/EditorBlueprintResources/StandardMacros.IsValid` _putactor
      (:`Is Valid`
        (`self.K2_AddActorWorldRotation` _putactor (struct :`Yaw` 90.0) false false)))))

(event `InputAxisKey|MouseX`
  (params (AxisValue :type "Float (single-precision)"))
  ;[1 1 1] 鼠标控制视角
  ;;[1 1 1] 右键旋转
  (`/Engine/EditorBlueprintResources/StandardMacros.Gate` true :!label _label_2
    (:`Exit`
      (`self.K2_AddActorLocalRotation` (`KismetMathLibrary.MakeRotator` 0.0 0.0 AxisValue)))))

(event `Key|RightMouseButton`
  (params (Key :type "Key Structure"))
  ;[1 1 1] 鼠标控制视角
  ;;[1 1 1] 右键旋转
  (:`Pressed`
    (goto _label_2 :!via `Open`))
  (:`Released`
    (goto _label_2 :!via `Close`)))

(event `InputAxisKey|MouseWheelAxis`
  (params (AxisValue :type "Float (single-precision)"))
  (bind _springarm (`self.SpringArm`))
  ;[1 1 1] 鼠标控制视角
  ;;[1 1 1] 滚轮前进
  (set `SpringArmComponent.TargetArmLength` (`KismetMathLibrary.FClamp` (+ (* AxisValue (`self.ForwarSpeed`) -1.0) (`SpringArmComponent.TargetArmLength` _springarm)) 0.0 60000.0) _springarm))

(fn `Control Target Move`
  (params (Target :type "/Game/Main/Blueprints/BP_Placeable0 Object Reference"))
  (bind _output_get (set `self.PutActor` Target))
  (`/Game/Main/Blueprints/BP_Placeable0.SetPlaced` _output_get false)
  (`self.SetGripsVisiblity` true)
  (`Widget.SetVisibility` (`self.UserUI`) "Hidden"))

(fn `GetMouseRay`
  (returns (OriginPosition :type "Vector Structure") (EndPosition :type "Vector Structure"))
  (bind _returnvalue (`GameplayStatics.GetPlayerController` 0))
  (bind (_locationx _locationy) (`PlayerController.GetMousePosition` _returnvalue))
  (bind (_worldposition _worlddirection) (`GameplayStatics.DeprojectScreenToWorld` _returnvalue (`KismetMathLibrary.MakeVector2D` _locationx _locationy)))
  (return _worldposition (+ _worldposition (* _worlddirection (* (`SpringArmComponent.TargetArmLength` (`self.SpringArm`)) 3.0)))))

(fn `Set Mouse To Actor`
  (params (Target :type "Actor Object Reference"))
  (bind _returnvalue (`GameplayStatics.GetPlayerController` 0))
  (bind (_screenposition _returnvalue_2) (`GameplayStatics.ProjectWorldToScreen` _returnvalue (`self.K2_GetActorLocation` Target) true))
  (`/Engine/EditorBlueprintResources/StandardMacros.IsValid` Target
    (:`Is Valid`
      (if _returnvalue_2
        (`PlayerController.SetMouseLocation` _returnvalue (`KismetMathLibrary.FTrunc` (`KismetMathLibrary.BreakVector2D` _screenposition)) (`KismetMathLibrary.FTrunc` (`.Y` (`KismetMathLibrary.BreakVector2D` _screenposition))))))))

(fn `SetGripsVisiblity`
  (params (Value :type Boolean))
  (bind _outactors (`GameplayStatics.GetAllActorsOfClass` "/Game/Main/Blueprints/Placeables/BP_Floor.BP_Floor_C"))
  (for _array_element _outactors
    (`/Game/Main/Blueprints/Placeables/BP_Floor.SetGripVisiblity` _array_element Value)))

(fn `UserConstructionScript`)