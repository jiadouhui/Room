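; BP_Placeable is an actor that provides a grid of placement cells over its PlaceableArea box.
; On BeginPlay it divides the box into evenly spaced rows and columns, adding a flat, hidden Paper sprite with the Grid collision profile for each cell.
; SetGridVisable shows or hides the stored cells, using overlap queries to keep any cell occupied by an actor other than its owner hidden.
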(event Custom|SetGridVisable
  (params (IsHidden :type Boolean))
  ;[1 1 1] 将可放置的格子放置
  (for _array_element (Variables|Default|GetGrids)
    (Development|SetHiddeninGame _array_element (or (!= (Utilities|Array|Length (Collision|GetOverlappingActors _array_element 0 :!class /Script/Engine.PrimitiveComponent)) (Math|Integer|SelectInt 1 0 (Utilities|Array|ContainsItem (Collision|GetOverlappingActors _array_element 0 :!class /Script/Engine.PrimitiveComponent) (Components|GetOwner _array_element)))) IsHidden) false)))

(event EventBeginPlay
  (bind _placeablearea (Variables|Default|GetPlaceableArea))
  (bind _returnvalue (Components|Box|GetUnscaledBoxExtent _placeablearea))
  (bind (_x _y) (Math|Vector|BreakVector _returnvalue))
  (bind (_row _colum) (|GetRectSplitNum (Math|Vector2D|MakeVector2D _x _y) 25.0))
  (|CallParentFunction)
  (Utilities|FlowControl|Sequence
    (:then_0
      ;[1 1 1] 生成格子
      (for _index (range 1 _row)
        (for _index_2 (range 1 _colum)
          (bind _returnvalue_2 (AddComponent|AddPaperSpriteComponent false (Math|Transform|MakeTransform (|GetGridLocation (Utilities|Operators|Subtract (Variables|/Script/Engine.SceneComponent|GetRelativeLocation _placeablearea) _returnvalue "(X=25.000000,Y=25.000000)") _index _index_2) "0.000000,0.000000,90.000000" "0.900000,0.900000,0.900000")))
          (Utilities|FlowControl|Sequence
            (:then_0
              ;[1 1 1] 添加数组
              (Utilities|Array|Add (Variables|Default|GetGrids) _returnvalue_2))
            (:then_1
              ;[1 1 1] 设置属性
              (Rendering|Components|Sprite|SetSprite _returnvalue_2 0)
              (Development|SetHiddeninGame _returnvalue_2 true false)
              (Collision|SetCollisionProfileName _returnvalue_2 "Grid" true :!class /Script/Engine.PrimitiveComponent))))))))

(fn ConstructionScript
  (|CallParentFunction))