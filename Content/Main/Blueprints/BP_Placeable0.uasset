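; Placeable grid object that can be moved, placed and removed through a 3D select-button widget.
; While moving, Tick traces up from "Placement"-tagged components to collect grid cells, tinting a spawned flash-mesh copy green or red.
; SetPlaced hides those cells and disables their collision, and destruction restores them.
; A RenderCamera showing only this object feeds a render target into a dynamic UI material for previews.
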(event `DestroySelf`
  ;[1 1 1] 点击删除时删除自身
  (`self.K2_DestroyActor`))

(event `self.ReceiveBeginPlay`
  (`self.SetGripVisiblity` false)
  (bind _returnvalue (`|CreateWidget` "/Game/Main/Blueprints/UI/BP_SelectBtn.BP_SelectBtn_C"))
  (bind _output_get (set `self.SelectUI` _returnvalue))
  (`|ExecutionSequence`
    (:`then_0`
      ;[1 1 1] 将生成的Widget显示到3D上
      (`WidgetComponent.SetWidget` (`self.Widget`) _output_get))
    (:`then_1`
      ;[1 1 1] 点击删除时删除自身
      (add `/Game/Main/Blueprints/UI/BP_SelectBtn.ClickRemove` _output_get (delegate `DestroySelf`)))
    (:`then_2`
      ;[1 1 1] 点击设置时关闭UI
      (add `/Game/Main/Blueprints/UI/BP_SelectBtn.ClickMove` _output_get (delegate `HideSelectBtns`)))))

(event `HideSelectBtns`
  ;[1 1 1] 点击设置时关闭UI
  (`SceneComponent.SetVisibility` (`self.Widget`) false false)
  (`self.DestroyVaildActor` (`self.SelectFlashMesh`)))

(event `self.ReceiveTick`
  (params (DeltaSeconds :type "Float (single-precision)"))
  (bind _moveflashmesh (`self.MoveFlashMesh`))
  (bind _placedgrip (`self.PlacedGrip`))
  ;[1 1 1] 检测是否在可放置位置
  (`/Engine/EditorBlueprintResources/StandardMacros.IsValid` (`self.MoveFlashMesh`)
    (:`Is Valid`
      (`KismetArrayLibrary.Array_Clear` (`self.PlacedGrip`))
      (for _array_element (`self.GetComponentsByTag` "/Script/Engine.SceneComponent" "Placement")
        (bind _returnvalue (`SceneComponent.K2_GetComponentLocation` _array_element))
        (bind (_outhit _returnvalue_2) (`KismetSystemLibrary.LineTraceSingle` _returnvalue (+ _returnvalue (* (`KismetMathLibrary.Vector_Up`) 10.0)) "TraceTypeQuery2"))
        (bind _output_get (set `self.CanPlace` _returnvalue_2))
        (if _output_get
          (set `/Game/Main/Blueprints/BP_FlashStaticMesh.Color` (0.0 1.0 0.0) _moveflashmesh)
          (`KismetArrayLibrary.Array_Add` _placedgrip (`.HitComponent` (`GameplayStatics.BreakHitResult` _outhit)))
          (else
            (set `/Game/Main/Blueprints/BP_FlashStaticMesh.Color` (0.6 0.0 0.0) _moveflashmesh)
            (`KismetArrayLibrary.Array_Clear` _placedgrip)
            (break)))))))

(event `SetFlashEnable`
  (params (Value :type Boolean))
  ;[1 1 1] 闪烁函数
  (if Value
    (bind _value (`self.Spawn Flash Mesh`))
    (bind _output_get (set `self.MoveFlashMesh` _value))
    (`self.K2_AttachToActor` _output_get self "None" "KeepWorld" "KeepWorld" "KeepWorld" true)
    (else
      (`self.DestroyVaildActor` (`self.MoveFlashMesh`)))))

(event `SetGripVisiblity`
  (params (Value :type Boolean))
  ;[1 1 1] 格子显示开关
  (for _array_element (`self.K2_GetComponentsByClass` "/Script/Paper2D.PaperSpriteComponent")
    (`SceneComponent.SetVisibility` _array_element (and Value (`|EnumEquality` (`PrimitiveComponent.GetCollisionEnabled` _array_element) "QueryOnly")) true)))

(event `SetVisiblity`
  (params (Value :type Boolean))
  (bind _returnvalue (not Value))
  ;[1 1 1] 自身显示隐藏
  (`self.SetActorHiddenInGame` _returnvalue)
  (for _array_element (`self.GetAttachedActors` true)
    (`self.SetActorHiddenInGame` _array_element _returnvalue)))

(event `self.ReceiveDestroyed`
  ;[1 1 1] 销毁事件
  (`|ExecutionSequence`
    (:`then_0`
      ;;[1 1 1] 将闪烁对象一并删除
      (`self.DestroyVaildActor` (`self.MoveFlashMesh`)))
    (:`then_1`
      (`self.DestroyVaildActor` (`self.SelectFlashMesh`)))
    (:`then_2`
      ;;[1 1 1] 恢复格子碰撞检测
      (for _array_element (`self.PlacedGrip`)
        (`PrimitiveComponent.SetCollisionEnabled` _array_element "QueryOnly")
        (`SceneComponent.SetHiddenInGame` _array_element false false)))))

(fn `GetCanPlace`
  (returns (Value :type Boolean))
  (return (and (`self.CanPlace`) (not (`self.bHidden`)))))

(fn `GetRenderUIMaterial`
  (returns (Value :type "MaterialInterface Object Reference"))
  (bind _returnvalue (`KismetRenderingLibrary.CreateRenderTarget2D` 1080 1080 "RTF_RGBA32f"))
  (`|ExecutionSequence`
    (:`then_0`
      (bind _output_get (set `SceneCaptureComponent2D.TextureTarget` _returnvalue (`self.RenderCamera`))))
    (:`then_1`
      (bind _returnvalue_2 (`KismetMaterialLibrary.CreateDynamicMaterialInstance` "/Game/Main/Materials/Mat_UI.Mat_UI"))
      (`|ExecutionSequence`
        (:`then_0`
          (`MaterialInstanceDynamic.SetTextureParameterValue` _returnvalue_2 "RenderTarget" _output_get))
        (:`then_1`
          (return _returnvalue_2))))))

(fn `Set SelectBtnsIVisiblity `
  (params (Value :type Boolean) (Event :type "Delegate (by ref)"))
  (bind _widget (`self.Widget`))
  (bind _selectui (`self.SelectUI`))
  ;[1 1 1] Comment
  (`|ExecutionSequence`
    (:`then_0`
      (`SceneComponent.SetVisibility` _widget Value false))
    (:`then_1`
      (if Value
        (add `/Game/Main/Blueprints/UI/BP_SelectBtn.ClickMove` _selectui Event)
        (if (not (`SceneComponent.bHiddenInGame` _widget))
          (bind _value (`self.Spawn Flash Mesh`))
          (set `self.SelectFlashMesh` _value))
        (else
          (remove `/Game/Main/Blueprints/UI/BP_SelectBtn.ClickMove` _selectui Event)
          (`self.DestroyVaildActor` (`self.SelectFlashMesh`)))))))

(fn `SetPlaced`
  (params (Value :type Boolean))
  (locals (MeshCollisionType :type "ECollisionEnabled Enum") (GridCollisionType :type "ECollisionEnabled Enum"))
  (`|ExecutionSequence`
    (:`then_0`
      (if Value
        ;[1 1 1] 放置状态的碰撞类型
        (set `local.GridCollisionType` "NoCollision")
        (set `local.MeshCollisionType` "QueryAndPhysics")
        (else
          ;[1 1 1] 移动状态的碰撞类型
          (set `local.GridCollisionType` "QueryOnly")
          (set `local.MeshCollisionType` "NoCollision"))))
    (:`then_1`
      (`/Game/Main/Blueprints/Placeables/BP_Floor.SetFlashEnable` (not Value))
      (for _array_element (`self.PlacedGrip`)
        (`|ExecutionSequence`
          (:`then_0`
            (`PrimitiveComponent.SetCollisionEnabled` _array_element (`local.GridCollisionType`)))
          (:`then_1`
            (`SceneComponent.SetHiddenInGame` _array_element Value false)))))))

(fn `Spawn Flash Mesh`
  (returns (Value :type "/Game/Main/Blueprints/BP_FlashStaticMesh Object Reference"))
  (bind _staticmesh (`self.StaticMesh`))
  (bind (_returnvalue_location _returnvalue_rotation) (`KismetMathLibrary.BreakTransform` (`SceneComponent.K2_GetComponentToWorld` _staticmesh)))
  (bind _returnvalue (`|SpawnActorFromClass` "/Game/Main/Blueprints/BP_FlashStaticMesh.BP_FlashStaticMesh_C" (`KismetMathLibrary.MakeTransform` _returnvalue_location _returnvalue_rotation (* (`SceneComponent.K2_GetComponentScale` _staticmesh) 1.01)) "Undefined" "MultiplyWithRoot" null null))
  (`|ExecutionSequence`
    (:`then_0`
      (`/Game/Main/Blueprints/BP_FlashStaticMesh.SetStaticMesh` _returnvalue (`StaticMeshComponent.StaticMesh` _staticmesh)))
    (:`then_1`
      (return _returnvalue))))

(fn `UserConstructionScript`
  (bind _rendercamera (`self.RenderCamera`))
  (set `SceneCaptureComponent.ShowOnlyActors` (`|MakeArray` self :!type "Actor Object Reference") _rendercamera)
  (`SceneCaptureComponent.ShowOnlyComponent` _rendercamera (`self.StaticMesh`)))