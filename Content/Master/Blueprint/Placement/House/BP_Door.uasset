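; BP_Door is a placeable house door that swings open when something overlaps its trigger and closes when an overlap ends.
; The overlapping component's side in trigger-local space picks a 90-degree swing direction, so the door turns according to the approach side.
; The RotateTime timeline lerps the door's yaw and reverses to close.
; A gate blocks opening from StartMove until StopMove, while closing is ungated.
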(event `self.ReceiveBeginPlay`
  (`parent.ReceiveBeginPlay`)
  (`self.CastToFlashMaterials` (`self.FlashDoor`)))

(event `self.Trigger.OnComponentBeginOverlap`
  (params (OverlappedComponent :type "PrimitiveComponent Object Reference") (OtherActor :type "Actor Object Reference") (OtherComp :type "PrimitiveComponent Object Reference") (OtherBodyIndex :type Integer) (bFromSweep :type Boolean) (SweepResult :type "HitResult Structure (by ref)"))
  (bind (_relativerotation_roll _relativerotation_pitch _relativerotation_yaw) (`KismetMathLibrary.BreakRotator` (`SceneComponent.RelativeRotation` (`self.Door`))))
  (`/Engine/EditorBlueprintResources/StandardMacros.Gate` false :!label _label
    (:`Exit`
      (if (not (`self.IsOpen`))
        (set `self.TargetAngle` (* (`KismetMathLibrary.SignOfFloat` (.y (.location (`KismetMathLibrary.MakeRelativeTransform` (`SceneComponent.K2_GetComponentToWorld` OtherComp) (`SceneComponent.K2_GetComponentToWorld` (`self.Trigger`)))))) 90.0))
        (set `self.StartAngle` _relativerotation_yaw)
        (set `self.IsOpen` true)
        (bind (_direction _program) (`Timeline|RotateTime` :!label _label_2)
          (:`Update`
            (`SceneComponent.K2_SetRelativeRotation` (`self.Door`) (`KismetMathLibrary.MakeRotator` 0.0 0.0 (`KismetMathLibrary.Lerp` (`self.StartAngle`) (`self.TargetAngle`) _program)) false false)))))))

(event `self.StopMove`
  (`parent.StopMove`)
  (goto _label :!via `Open`))

(event `self.StartMove`
  (`parent.StartMove`)
  (goto _label :!via `Close`))

(event `self.Trigger.OnComponentEndOverlap`
  (params (OverlappedComponent :type "PrimitiveComponent Object Reference") (OtherActor :type "Actor Object Reference") (OtherComp :type "PrimitiveComponent Object Reference") (OtherBodyIndex :type Integer))
  (if (`self.IsOpen`)
    (set `self.IsOpen` false)
    (goto _label_2 :!via `Reverse`)))

(fn `UserConstructionScript`
  (`parent.UserConstructionScript`))