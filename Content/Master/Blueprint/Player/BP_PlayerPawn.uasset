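; VR player pawn, with mouse aim and look, for selecting, spawning, moving, rotating and deleting BP_Placement objects on placeable grid cells.
; Enhanced Input drives movement, snap turning and widget interaction, swapping preview and setting mapping contexts during placement.
; Niagara lines show UI, selection and projectile-arc placement traces, gated to avoid clashing with UI presses.
; Tick traces from the selected object to the widget to position the info panel's arrow.
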(event `self.ReceiveBeginPlay`
  (bind _panelcontroller (`self.PanelController`))
  (`|ExecutionSequence`
    (:`then_0`
      ;[1 1 1] VR模式调整摄像头
      (if (`HeadMountedDisplayFunctionLibrary.IsHeadMountedDisplayEnabled`)
        (`HeadMountedDisplayFunctionLibrary.SetTrackingOrigin` "Floor")
        (`SceneComponent.K2_SetRelativeLocation` (`self.Root`) (0.0 0.0 -92.0) false false)))
    (:`then_1`
      ;[1 1 1] 初始使用选择输入
      (`EnhancedInputSubsystemInterface.AddMappingContext` (pcsubsystem `EnhancedInputLocalPlayerSubsystem` (`GameplayStatics.GetPlayerController` 0)) "/Game/Master/Input/IMC_VRPreview.IMC_VRPreview" 0 (struct)))
    (:`then_2`
      ;[1 1 1] 初始化UI
      (bind _returnvalue (`|CreateWidget` "/Game/Master/UIKit/UI_InfoPanel.UI_InfoPanel_C"))
      (bind _output_get (set `self.InfoPanel` _returnvalue))
      (`PanelControllerComponent.RegisterPanel` _panelcontroller _output_get)
      (`WidgetComponent.SetWidget` (`self.MasterWidget`) (`PanelControllerComponent.PanelSpace` _panelcontroller)))
    (:`then_3`
      (bind _returnvalue_2 (`|CreateWidget` "/Game/Master/UIKit/UI_Message.UI_Message_C"))
      (bind _output_get_2 (set `self.MessageUI` _returnvalue_2))
      (`WidgetComponent.SetWidget` (`self.MessageWidget`) _output_get_2))))

(event `self.ReceiveTick`
  (params (DeltaSeconds :type "Float (single-precision)"))
  (bind _panelcontroller (`self.PanelController`))
  (`|ExecutionSequence`
    (:`then_0`
      ;[1 1 1] 绘画UI射线
      (`self.TraceUILine` (`self.RightWidgetInteraction`) (`self.RightUILineNiagara`))
      (`self.TraceUILine` (`self.LeftWidgetInteraction`) (`self.LeftUILineNiagara`)))
    (:`then_1`
      ;[1 1 1] 消息UI显示
      ;;[0.07451 0.07451 0.07451] 是否符合显示条件
      (bind _selectactor (`self.SelectActor`)
        (:`then`
          (if (`self.WasRecentlyRendered` _selectactor 0.1)
            (bind (_issuccess _pivot) (`self.TraceCrossUI` (`SceneComponent.K2_GetComponentLocation` (`/Game/Master/Blueprint/Placement/BP_Placement.Occupied` _selectactor))))
            (if _issuccess
              ;;[0.07451 0.07451 0.07451] 设置显示位置
              (`/Game/Master/UIKit/UI_InfoPanel.SetArrowPoint` (`self.InfoPanel`) _pivot)
              (`PanelControllerComponent.PushUI` _panelcontroller "/Game/Master/UIKit/UI_InfoPanel.UI_InfoPanel_C")
              (else
                (if (not (`self.IsMoving`)) :!label _label
                  ;;[0.07451 0.07451 0.07451] 关闭UI显示
                  (set `self.SelectActor` null :!label _label_2))
                (`PanelControllerComponent.PopUI` _panelcontroller false)))
            (else
              (goto _label))))
        (:`else`)))))

(event `ClearSelect`
  ;[1 1 1] 消息UI显示
  (goto _label_2))

(event `Key|Tab`
  (params (Key :type "Key Structure"))
  (:`Pressed`
    (bind _isa (`/Engine/EditorBlueprintResources/StandardMacros.FlipFlop`)
      (:`A`
        _)
      (:`B`
        _))
    (`self.SetGridsVisiblity` _isa)))

(event `EnhancedInput|/Game/Master/Input/PC/IA_Point`
  (params (ActionValue :type Boolean) (ElapsedSeconds :type "Float (double-precision)") (TriggeredSeconds :type "Float (double-precision)") (InputAction :type "InputAction Object Reference" :default "/Game/Master/Input/PC/IA_Point.IA_Point"))
  (bind _returnvalue (`GameplayStatics.GetPlayerController` 0))
  (bind _right_motion (`self.Right Motion`))
  (bind (_locationx _locationy) (`PlayerController.GetMousePosition` _returnvalue))
  (bind (_worldposition _worlddirection) (`GameplayStatics.DeprojectScreenToWorld` _returnvalue (`KismetMathLibrary.MakeVector2D` _locationx _locationy)))
  ;[1 1 1] 鼠标瞄准
  (:`Triggered`
    (`SceneComponent.K2_SetWorldLocation` _right_motion _worldposition false false)
    (`SceneComponent.K2_SetWorldRotation` _right_motion (`KismetMathLibrary.Conv_VectorToRotator` (+ _worlddirection (* (`SceneComponent.GetUpVector` _right_motion) 0.5))) false false)))

(event `EnhancedInput|/Game/Master/Input/PC/IA_TurnLook`
  (params (ActionValue :type "Vector2D Structure") (ElapsedSeconds :type "Float (double-precision)") (TriggeredSeconds :type "Float (double-precision)") (InputAction :type "InputAction Object Reference" :default "/Game/Master/Input/PC/IA_TurnLook.IA_TurnLook"))
  (bind (_x _y) (`KismetMathLibrary.BreakVector2D` ActionValue))
  ;[1 1 1] 摄像机旋转
  (:`Triggered`
    (`/Engine/EditorBlueprintResources/StandardMacros.Gate` true :!label _label
      (:`Exit`
        (`SceneComponent.K2_AddRelativeRotation` (`self.Camera`) (`KismetMathLibrary.MakeRotator` 0.0 _y _x) false false)))))

(event `EnhancedInput|/Game/Master/Input/PC/IA_Turning`
  (params (ActionValue :type Boolean) (ElapsedSeconds :type "Float (double-precision)") (TriggeredSeconds :type "Float (double-precision)") (InputAction :type "InputAction Object Reference" :default "/Game/Master/Input/PC/IA_Turning.IA_Turning"))
  ;[1 1 1] 摄像机旋转
  (:`Started`
    (goto _label :!via `Open`))
  (:`Completed`
    (goto _label :!via `Close`)))

(event `/Game/Master/Blueprint/UIEvent/BP_IUIEvent.InvokeRotate`
  ;[1 1 1] 选中的物品旋转
  (bind _selectactor (`self.SelectActor`)
    (:`then`
      (`self.K2_AddActorWorldRotation` _selectactor (struct :`Yaw` 90.0) false false))
    (:`else`)))

(event `/Game/Master/Blueprint/UIEvent/BP_IUIEvent.OnInfoClosed`
  ;[1 1 1] 关闭消息面板
  (set `self.SelectActor` null))

(event `/Game/Master/Blueprint/UIEvent/BP_IUIEvent.InvokeRemoveSelect`
  ;[1 1 1] 删除选中物品
  (`self.K2_DestroyActor` (`self.SelectActor`))
  (`self.SetGridsVisiblity` true))

(event `/Game/Master/Blueprint/UIEvent/BP_IUIEvent.InvokeMove`
  (bind _returnvalue (pcsubsystem `EnhancedInputLocalPlayerSubsystem` (`GameplayStatics.GetPlayerController` 0)))
  ;[1 1 1] UI按钮移动物品
  (bind _selectactor (`self.SelectActor` :!label _label)
    (:`then`
      (`/Game/Master/Blueprint/Placement/BP_Placement.StartMove` _selectactor)
      (`self.SetGridsVisiblity` false)
      (set `self.IsMoving` true)
      (`EnhancedInputSubsystemInterface.RemoveMappingContext` _returnvalue "/Game/Master/Input/IMC_VRPreview.IMC_VRPreview" (struct))
      (`EnhancedInputSubsystemInterface.AddMappingContext` _returnvalue "/Game/Master/Input/IMC_VRSetting.IMC_VRSetting" 0 (struct))
      (`PanelControllerComponent.PushUI` (`self.PanelController`) "/Game/Master/UIKit/UI_InfoPanel.UI_InfoPanel_C"))
    (:`else`)))

(event `/Game/Master/Blueprint/UIEvent/BP_IUIEvent.SpawnPalcement`
  (params (Target :type "/Game/Master/Blueprint/BP_Interactivable Class Reference"))
  (bind _infopanel (`self.InfoPanel`))
  ;[1 1 1] 生成事件
  (bind (_placeable _returnvalue) (`self.GetForwardPlaceableArea`))
  (if _placeable
    (bind _returnvalue_2 (`|SpawnActorFromClass` Target (`KismetMathLibrary.MakeTransform` _returnvalue) "Undefined" "MultiplyWithRoot" null null))
    (bind _asbp_placement (cast `/Game/Master/Blueprint/Placement/BP_Placement` _returnvalue_2))
    (`self.FroceSelect` _asbp_placement)
    (set `Widget.Visibility` "Collapsed" (`/Game/Master/UIKit/UI_InfoPanel.CommandButtons` _infopanel))
    (set `Widget.Visibility` "Visible" (`/Game/Master/UIKit/UI_InfoPanel.OptionButtons` _infopanel))
    (goto _label)
    (else
      (`PanelControllerComponent.PopUI` (`self.PanelController`) false)
      (`/Game/Master/UIKit/UI_Message.Display` (`self.MessageUI`) "前方无多余空间生成"))))

(event `/Game/Master/Blueprint/UIEvent/BP_IUIEvent.ShowMessage`
  (params (Message :type Text))
  (`/Game/Master/UIKit/UI_Message.Display` (`self.MessageUI`) Message))

(event `EnhancedInput|/Game/Master/Input/Normal/IA_Turn`
  (params (ActionValue :type Boolean) (ElapsedSeconds :type "Float (double-precision)") (TriggeredSeconds :type "Float (double-precision)") (InputAction :type "InputAction Object Reference" :default "/Game/Master/Input/Normal/IA_Turn.IA_Turn"))
  (bind (_relativerotation_roll _relativerotation_pitch _relativerotation_yaw) (`KismetMathLibrary.BreakRotator` (`SceneComponent.RelativeRotation` (`self.Camera`))))
  ;[1 1 1] 90度旋转, 方向由摄像机左右决定
  (:`Triggered`
    (`self.K2_AddActorWorldRotation` (`KismetMathLibrary.MakeRotator` 0.0 0.0 (* (`KismetMathLibrary.SignOfFloat` _relativerotation_yaw) -90.0)))))

(event `EnhancedInput|/Game/Master/Input/Normal/IA_Move`
  (params (ActionValue :type "Vector2D Structure") (ElapsedSeconds :type "Float (double-precision)") (TriggeredSeconds :type "Float (double-precision)") (InputAction :type "InputAction Object Reference" :default "/Game/Master/Input/Normal/IA_Move.IA_Move"))
  (bind (_returnvalue_x _returnvalue_y) (`KismetMathLibrary.BreakVector2D` (* ActionValue 5.0)))
  (bind (_returnvalue_roll _returnvalue_pitch _returnvalue_yaw) (`KismetMathLibrary.BreakRotator` (`SceneComponent.K2_GetComponentRotation` (`self.Camera`))))
  (bind (_returnvalue_x_2 _returnvalue_y_2) (`KismetMathLibrary.BreakVector` (`KismetMathLibrary.GetForwardVector` (`KismetMathLibrary.MakeRotator` 0.0 0.0 _returnvalue_yaw))))
  (bind (_returnvalue_x_3 _returnvalue_y_3) (`KismetMathLibrary.BreakVector` (`KismetMathLibrary.GetRightVector` (`KismetMathLibrary.MakeRotator` 0.0 0.0 _returnvalue_yaw))))
  ;[1 1 1] 移动输入
  (:`Triggered`
    ;;[0.07451 0.07451 0.07451] 移动
    (bind _sweephitresult (`self.K2_AddActorWorldOffset` (+ (* _returnvalue_x (`KismetMathLibrary.MakeVector` _returnvalue_x_2 _returnvalue_y_2)) (* _returnvalue_y (`KismetMathLibrary.MakeVector` _returnvalue_x_3 _returnvalue_y_3))) true))
    ;;[0.07451 0.07451 0.07451] 撞到墙停止摄像机抖动
    (`self.SetCameraShake` (not (`GameplayStatics.BreakHitResult` _sweephitresult))))
  (:`Started`
    ;;[0.07451 0.07451 0.07451] 摄像机抖动
    (`self.SetCameraShake` true))
  (:`Completed`
    (`self.SetCameraShake` false)))

(event `EnhancedInput|/Game/Master/Input/Normal/IA_TriggerUI`
  (params (ActionValue :type Boolean) (ElapsedSeconds :type "Float (double-precision)") (TriggeredSeconds :type "Float (double-precision)") (InputAction :type "InputAction Object Reference" :default "/Game/Master/Input/Normal/IA_TriggerUI.IA_TriggerUI"))
  (bind _leftwidgetinteraction (`self.LeftWidgetInteraction`))
  (bind _rightwidgetinteraction (`self.RightWidgetInteraction`))
  ;[1 1 1] UI交互
  (:`Started`
    (`self.PointPress` _rightwidgetinteraction)
    (`self.PointPress` _leftwidgetinteraction))
  (:`Completed`
    (`self.PointRelease` _rightwidgetinteraction)
    (`self.PointRelease` _leftwidgetinteraction)))

(event `EnhancedInput|/Game/Master/Input/Normal/IA_Select`
  (params (ActionValue :type Boolean) (ElapsedSeconds :type "Float (double-precision)") (TriggeredSeconds :type "Float (double-precision)") (InputAction :type "InputAction Object Reference" :default "/Game/Master/Input/Normal/IA_Select.IA_Select"))
  (bind (_origion _end) (`self.GetForwardLine` (`self.RightWidgetInteraction`)))
  ;[1 1 1] 瞄准选择物品
  (:`Triggered`
    (`self.TraceInput` (`self.SelectLineNiagara`) :!label _label
      (:`OnTriggered`
        ;;[0.07451 0.07451 0.07451] 射线检测
        (bind (_outhit _returnvalue) (`KismetSystemLibrary.LineTraceSingleForObjects` _origion _end (`|MakeArray` "ObjectTypeQuery8" :!type "EObjectTypeQuery Enum")))
        (`|ExecutionSequence`
          (:`then_0`
            (bind (_bblockinghit _binitialoverlap _time _distance _location _impactpoint _normal _impactnormal _physmat _hitactor) (`GameplayStatics.BreakHitResult` _outhit))
            ;;[0.07451 0.07451 0.07451] 射线两点连线
            (`NiagaraDataInterfaceArrayFunctionLibrary.SetNiagaraArrayVector` (`self.SelectLineNiagara`) "User.PointArray" (`|MakeArray` _origion (`KismetMathLibrary.SelectVector` _location _end _returnvalue))))
          (:`then_1`
            ;;[0.07451 0.07451 0.07451] 记录选中对象
            (if _returnvalue
              (bind _asbp_placement (cast `/Game/Master/Blueprint/Placement/BP_Placement` _hitactor)
                (:`then`
                  (`self.FroceSelect` _asbp_placement))
                (:`CastFailed`
                  (`self.ClearSelect` :!label _label_2)))
              (else
                (goto _label_2))))))))
  (:`Completed`
    (goto _label :!via `Complete`)))

(event `/Game/Master/Blueprint/UIEvent/BP_IUIEvent.OnUITrigger`
  (bind _rightwidgetinteraction (`self.RightWidgetInteraction`))
  ;[1 1 1] 触发UI后需重新按下才能发射射线
  (`|ExecutionSequence`
    (:`then_0`
      (goto _label :!via `Disable`))
    (:`then_1`
      (goto _label_3 :!via `Disable`))))

(event `EnhancedInput|/Game/Master/Input/Setting/IA_Placed`
  (params (ActionValue :type Boolean) (ElapsedSeconds :type "Float (double-precision)") (TriggeredSeconds :type "Float (double-precision)") (InputAction :type "InputAction Object Reference" :default "/Game/Master/Input/Setting/IA_Placed.IA_Placed"))
  (bind _rightwidgetinteraction (`self.RightWidgetInteraction`))
  ;[1 1 1] 抛物线放置
  (:`Triggered`
    (`self.TraceInput` (`self.PlaceLineNiagara`) :!label _label_3
      (:`OnTriggered`
        ;;[0.07451 0.07451 0.07451] 绘画射线
        (bind (_outhit _outpathpositions _outlasttracedestination _returnvalue) (`GameplayStatics.Blueprint_PredictProjectilePath_ByObjectType` (`SceneComponent.K2_GetComponentLocation` _rightwidgetinteraction) (* (`SceneComponent.GetForwardVector` _rightwidgetinteraction) 650.0) true 3.6 (`|MakeArray` "ObjectTypeQuery7" :!type "EObjectTypeQuery Enum")))
        (`NiagaraDataInterfaceArrayFunctionLibrary.SetNiagaraArrayVector` (`self.PlaceLineNiagara`) "User.PointArray" _outpathpositions)
        ;;[0.07451 0.07451 0.07451] 移动预览落点
        (if _returnvalue
          (bind (_bblockinghit _binitialoverlap _time _distance _location _impactpoint _normal _impactnormal _physmat _hitactor _hitcomponent) (`GameplayStatics.BreakHitResult` _outhit))
          (if (not (`SceneComponent.bHiddenInGame` _hitcomponent))
            (bind _selectactor (`self.SelectActor`)
              (:`then`
                (`self.K2_SetActorLocation` _selectactor (- (`SceneComponent.K2_GetComponentLocation` _hitcomponent) (0.0 0.0 10.0)) false false))
              (:`else`)))))))
  (:`Completed`
    (goto _label_3 :!via `Complete`)))

(event `EnhancedInput|/Game/Master/Input/Normal/IA_Meun`
  (params (ActionValue :type Boolean) (ElapsedSeconds :type "Float (double-precision)") (TriggeredSeconds :type "Float (double-precision)") (InputAction :type "InputAction Object Reference" :default "/Game/Master/Input/Normal/IA_Meun.IA_Meun"))
  ;[1 1 1] 打开菜单
  (:`Triggered`
    (`PanelControllerComponent.PushUI` (`self.PanelController`) "/Game/Master/UIKit/Menu/UI_MenuPanel.UI_MenuPanel_C")
    (set `self.SelectActor` null)))

(fn `FroceSelect`
  (params (SelectActor :type "/Game/Master/Blueprint/Placement/BP_Placement Object Reference"))
  (bind _output_get (set `self.SelectActor` SelectActor))
  (`/Game/Master/UIKit/UI_InfoPanel.SetTitle` (`self.InfoPanel`) (`/Game/Master/Blueprint/BP_Interactivable.Name` _output_get)))

(fn `GetForwardLine`
  (params (Target :type "SceneComponent Object Reference") (Distance :type "Float (single-precision)" :default 500.0))
  (returns (Origion :type "Vector Structure") (End :type "Vector Structure"))
  (bind _returnvalue (`SceneComponent.K2_GetComponentLocation` Target))
  (return _returnvalue (+ _returnvalue (* (`SceneComponent.GetForwardVector` Target) Distance))))

(fn `GetForwardPlaceableArea`
  (returns (Placeable :type Boolean) (ReturnValue :type "Vector Structure"))
  (bind _camera (`self.Camera`))
  (bind (_returnvalue_roll _returnvalue_pitch _returnvalue_yaw) (`KismetMathLibrary.BreakRotator` (`SceneComponent.K2_GetComponentRotation` _camera)))
  (bind _returnvalue (+ (`SceneComponent.K2_GetComponentLocation` _camera) (* (`KismetMathLibrary.GetForwardVector` (`KismetMathLibrary.MakeRotator` 0.0 0.0 _returnvalue_yaw)) 250.0)))
  (`self.SetGridsVisiblity` false)
  (bind _outhits (`KismetSystemLibrary.BoxTraceMultiForObjects` _returnvalue (- _returnvalue (0.0 0.0 500.0)) (75.0 75.0 75.0) (`KismetMathLibrary.MakeRotator` 0.0 0.0 _returnvalue_yaw) (`|MakeArray` "ObjectTypeQuery7" :!type "EObjectTypeQuery Enum")))
  (for _array_element _outhits
    (bind (_bblockinghit _binitialoverlap _time _distance _location _impactpoint _normal _impactnormal _physmat _hitactor _hitcomponent) (`GameplayStatics.BreakHitResult` _array_element))
    ;[1 1 1] 没隐藏的格子为可放置格子
    (if (not (`SceneComponent.bHiddenInGame` _hitcomponent))
      (return true (- (`SceneComponent.K2_GetComponentLocation` _hitcomponent) (0.0 0.0 10.0)))))
  (`self.SetGridsVisiblity` true)
  (return false (0.0 0.0 0.0)))

(fn `GetMouseRay`
  (returns (OriginPosition :type "Vector Structure") (Direction :type "Vector Structure"))
  (bind _returnvalue (`GameplayStatics.GetPlayerController` 0))
  (bind (_locationx _locationy) (`PlayerController.GetMousePosition` _returnvalue))
  (bind (_worldposition _worlddirection) (`GameplayStatics.DeprojectScreenToWorld` _returnvalue (`KismetMathLibrary.MakeVector2D` _locationx _locationy)))
  (return _worldposition (+ _worldposition (* _worlddirection 500.0))))

(fn `IsTraceUI`
  (returns (ReturnValue :type Boolean))
  (bind _returnvalue (`PanelSpaceWidget.GetTopPanel` (`PanelControllerComponent.PanelSpace` (`self.PanelController`))))
  (`|ExecutionSequence`
    (:`then_0`
      (`/Engine/EditorBlueprintResources/StandardMacros.IsValid` _returnvalue
        (:`Is Valid`
          (bind _returnvalue_2 (message `/Game/Master/UIKit/BP_IHitablePointer.IsHit` _returnvalue))
          (return (and _returnvalue_2 (`|EnumEquality` (`UIPanelWidget.State` _returnvalue) "Display"))))))
    (:`then_1`
      (return false))))

(fn `PointPress`
  (params (WidgetInteraction :type "WidgetInteractionComponent Object Reference"))
  (`WidgetInteractionComponent.PressPointerKey` WidgetInteraction "LeftMouseButton")
  (`WidgetInteractionComponent.PressPointerKey` WidgetInteraction "RightMouseButton"))

(fn `PointRelease`
  (params (WidgetInteraction :type "WidgetInteractionComponent Object Reference"))
  (`WidgetInteractionComponent.ReleasePointerKey` WidgetInteraction "LeftMouseButton")
  (`WidgetInteractionComponent.ReleasePointerKey` WidgetInteraction "RightMouseButton"))

(fn `SavePlaced`
  (returns (IsSuccess :type Boolean))
  (bind _selectactor (`self.SelectActor`))
  (bind _returnvalue (pcsubsystem `EnhancedInputLocalPlayerSubsystem` (`GameplayStatics.GetPlayerController` 0)))
  (if (`/Game/Master/Blueprint/Placement/BP_Placement.IsVaildPlace` _selectactor)
    (`/Game/Master/Blueprint/Placement/BP_Placement.StopMove` _selectactor)
    (set `Widget.Visibility` "Collapsed" (`/Game/Master/UIKit/UI_InfoPanel.OptionButtons` (`self.InfoPanel`)))
    (set `self.SelectActor` null)
    (`self.SetGridsVisiblity` true)
    (`EnhancedInputSubsystemInterface.RemoveMappingContext` _returnvalue "/Game/Master/Input/IMC_VRSetting.IMC_VRSetting" (struct))
    (`EnhancedInputSubsystemInterface.AddMappingContext` _returnvalue "/Game/Master/Input/IMC_VRPreview.IMC_VRPreview" 0 (struct))
    (return true)
    (else
      (return false))))

(fn `SetCameraShake`
  (params (Enable :type Boolean))
  (bind _isshaking (`self.IsShaking`))
  (bind _moveshake (`self.MoveShake`))
  (if (!= Enable _isshaking)
    (bind _output_get (set `self.IsShaking` (not _isshaking)))
    (if _output_get
      (`CameraShakeSourceComponent.Start` _moveshake)
      (else
        (`CameraShakeSourceComponent.StopAllCameraShakes` _moveshake true)))))

(fn `SetGridsVisiblity`
  (params (IsHidden :type Boolean))
  (bind _outactors (`GameplayStatics.GetAllActorsOfClass` "/Game/Master/Blueprint/Placement/Placeable/BP_Placeable.BP_Placeable_C"))
  (for _array_element _outactors
    (`/Game/Master/Blueprint/Placement/Placeable/BP_Placeable.SetGridVisable` _array_element IsHidden)))

(fn `TraceCrossUI`
  (params (Origion :type "Vector Structure") (MaxDistance :type "Float (double-precision)" :default 750.0))
  (returns (IsSuccess :type Boolean) (Pivot :type "Vector2D Structure"))
  (bind _returnvalue (`SceneComponent.K2_GetComponentLocation` (`self.Camera`)))
  (if (> MaxDistance (`KismetMathLibrary.Vector_Distance` Origion _returnvalue))
    ;[1 1 1] 检测是否射到UI
    (bind (_outhit _returnvalue_2) (`KismetSystemLibrary.LineTraceSingleForObjects` :`Start` Origion :`End` _returnvalue :`ObjectTypes` (`|MakeArray` "ObjectTypeQuery9" :!type "EObjectTypeQuery Enum") :`bIgnoreSelf` false))
    (if _returnvalue_2
      (bind (_bblockinghit _binitialoverlap _time _distance _location _impactpoint _normal _impactnormal _physmat _hitactor _hitcomponent) (`GameplayStatics.BreakHitResult` _outhit))
      (bind _aswidget_component (cast `WidgetComponent` _hitcomponent)
        (:`then`
          (bind _returnvalue_3 (`SceneComponent.K2_GetComponentToWorld` _aswidget_component))
          (bind _returnvalue_4 (`KismetMathLibrary.MakeRelativeTransform` _returnvalue_3 (`KismetMathLibrary.MakeTransform` _location (.rotation _returnvalue_3) (.scale _returnvalue_3))))
          ;[1 1 1] 计算中心偏移点
          (return true (/ (`KismetMathLibrary.MakeVector2D` (.y (.location _returnvalue_4)) (.z (.location _returnvalue_4))) (* (`WidgetComponent.GetDrawSize` _aswidget_component) 0.5))))
        (:`CastFailed`
          _))))
  (return false (0.0 0.0)))

(fn `TraceUILine`
  (params (Direction :type "SceneComponent Object Reference") (LineNiagara :type "NiagaraComponent Object Reference"))
  (bind (_origion _end) (`self.GetForwardLine` Direction 300.0))
  (bind (_outhit _returnvalue) (`KismetSystemLibrary.LineTraceSingleForObjects` :`Start` _origion :`End` _end :`ObjectTypes` (`|MakeArray` "ObjectTypeQuery9" :!type "EObjectTypeQuery Enum") :`bIgnoreSelf` false))
  (bind _returnvalue_2 (and _returnvalue (`self.IsTraceUI`)))
  (`SceneComponent.SetHiddenInGame` LineNiagara (not _returnvalue_2) false)
  (if _returnvalue_2
    (`NiagaraDataInterfaceArrayFunctionLibrary.SetNiagaraArrayVector` LineNiagara "User.PointArray" (`|MakeArray` (`.Location` (`GameplayStatics.BreakHitResult` _outhit)) _origion))))

(fn `UserConstructionScript`)