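; Game mode that builds the starting floor area at BeginPlay and shows the mouse cursor.
; Two nested loops over Width and Height spawn BP_Floor actors on a 100-unit grid, marking each as placed.
; GetIndex turns each size into a symmetric index range around zero, centering the grid on the world origin, with Width running along Y and Height along X.
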(event `self.ReceiveBeginPlay`
  (bind (_first _last) (`self.GetIndex` (`self.Height`)))
  (bind (_first_2 _last_2) (`self.GetIndex` (`self.Width`)))
  (set `PlayerController.bShowMouseCursor` true (`GameplayStatics.GetPlayerController` 0))
  ;[1 1 1] 生成地板区域
  (for _index (range _first_2 (+ _last_2 1))
    (for _index_2 (range _first (+ _last 1))
      (bind _returnvalue (`|SpawnActorFromClass` "/Game/Main/Blueprints/Placeables/BP_Floor.BP_Floor_C" (`KismetMathLibrary.MakeTransform` (`KismetMathLibrary.MakeVector` (* _index_2 100.0) (* _index 100.0))) "Undefined" "OverrideRootScale" null null))
      (`/Game/Main/Blueprints/BP_Placeable0.SetPlaced` _returnvalue true))))

(fn `GetIndex`
  (params (Target :type Integer))
  (returns (First :type Integer) (Last :type Integer))
  (bind _returnvalue (/ Target 2))
  (return (* _returnvalue -1) _returnvalue))

(fn `UserConstructionScript`)